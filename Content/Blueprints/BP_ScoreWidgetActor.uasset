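; BP_ScoreWidgetActor is an actor holding a minutes-and-seconds countdown, apparently for a ball game's score display.
; StartTimer steps Sec and Min down by one second per call and stops at zero.
; The logic to find BP_Ball, start the looping timer and pause it on goals is disconnected, so nothing here starts the countdown.
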(event EventBeginPlay)

(event Collision|EventActorBeginOverlap
  (params (OtherActor :type Actor%20Object%20Reference)))

(event EventTick
  (params (DeltaSeconds :type Float%20%28single-precision%29)))

(fn ConstructionScript)

(fn StartTimer
  (if (== (Variables|Default|GetSec) 0)
    (if (not (== (Variables|Default|GetMin) 0))
      (Variables|Default|SetSec 59)
      (Variables|Default|SetMin (- (Variables|Default|GetMin) 1)))
    (else
      (Variables|Default|SetSec (- (Variables|Default|GetSec) 1)))))